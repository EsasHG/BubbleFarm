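; BP_Bubble is an oxygen bubble that grows or shrinks with the net oxygen production of actors inside it.
; It sums OxygenProduction from BP_OxygenComponent on initial overlaps a tick after BeginPlay, then adjusts the total on begin and end overlap.
; Overlaps also notify pc_mainCharacter when it enters or leaves.
; Tick adds that total times delta time to actor scale and shows GameOverMenu once X scale reaches zero.
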(event EventBeginPlay
  (Utilities|FlowControl|DelayUntilNextTick)
  (for _array_element (Collision|GetOverlappingActors 0 :!class /Script/Engine.Actor)
    (if (Utilities|IsValid (Actor|GetComponentbyClass _array_element "/Game/OURSTUFF/BP_OxygenComponent.BP_OxygenComponent_C"))
      (Variables|Default|SetTotalOxygenProduction (+ (Variables|/Game/OURSTUFF/BP_OxygenComponent.BP_OxygenComponent_C|GetOxygenProduction (Actor|GetComponentbyClass _array_element "/Game/OURSTUFF/BP_OxygenComponent.BP_OxygenComponent_C")) (Variables|Default|GetTotalOxygenProduction))))))

(event Collision|EventActorBeginOverlap
  (params (OtherActor :type Actor%20Object%20Reference))
  (bind _returnvalue (Actor|GetComponentbyClass OtherActor "/Game/OURSTUFF/BP_OxygenComponent.BP_OxygenComponent_C"))
  (bind (_aspc_main_character _bsuccess) (Utilities|Casting|CastTopc_mainCharacter OtherActor))
  (if (Utilities|IsValid _returnvalue)
    (Variables|Default|SetTotalOxygenProduction (+ (Variables|Default|GetTotalOxygenProduction) (Variables|/Game/OURSTUFF/BP_OxygenComponent.BP_OxygenComponent_C|GetOxygenProduction _returnvalue)))
    (if _bsuccess
      (Default|EnteredBubble _aspc_main_character))))

(event EventTick
  (params (DeltaSeconds :type Float%20%28single-precision%29))
  (bind _returnvalue (Transformation|GetActorScale3D))
  (bind _totaloxygenproduction (Variables|Default|GetTotalOxygenProduction))
  (bind _returnvalue_2 (* DeltaSeconds _totaloxygenproduction))
  (bind _returnvalue_3 (+ _returnvalue _returnvalue_2))
  ;[0.15 0.15 0.15 0.5] Bubble shrinking logic
  (Transformation|SetActorScale3D (Math|Vector|MakeVector (.x _returnvalue_3) (.y _returnvalue_3) (.z _returnvalue_3)))
  (if (<= (.x (Transformation|GetActorScale3D)) 0.0)
    (bind _returnvalue_4 (UserInterface|CreateWidget "/Game/OURSTUFF/UI/GameOverMenu.GameOverMenu_C"))
    (UserInterface|Viewport|AddtoViewport _returnvalue_4 0)))

(event Collision|EventActorEndOverlap
  (params (OtherActor :type Actor%20Object%20Reference))
  (bind _returnvalue (Actor|GetComponentbyClass OtherActor "/Game/OURSTUFF/BP_OxygenComponent.BP_OxygenComponent_C"))
  (bind (_aspc_main_character _bsuccess) (Utilities|Casting|CastTopc_mainCharacter OtherActor))
  (if (Utilities|IsValid _returnvalue)
    (Variables|Default|SetTotalOxygenProduction (- (Variables|Default|GetTotalOxygenProduction) (Variables|/Game/OURSTUFF/BP_OxygenComponent.BP_OxygenComponent_C|GetOxygenProduction _returnvalue)))
    (if _bsuccess
      (Default|LeftBubble _aspc_main_character))))

(fn ConstructionScript)