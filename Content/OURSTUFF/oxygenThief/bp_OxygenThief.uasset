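; Oxygen thief actor that moves in 2D at Speed, apparently meant to approach the edge of the BP_Bubble.
; BeginPlay caches the bubble one tick after starting.
; Tick computes the nearest point on the bubble's sphere radius, then steps X and Y by Speed and delta time.
; Step direction and 10-unit threshold use that point's absolute world position, rather than its offset from the thief.
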(event EventBeginPlay
  (Utilities|FlowControl|DelayUntilNextTick)
  (bind _returnvalue (Actor|GetActorOfClass "/Game/TopDown/Blueprints/Bubble/BP_Bubble.BP_Bubble_C"))
  (Variables|Default|SetBubble _returnvalue))

(event Collision|EventActorBeginOverlap
  (params (OtherActor :type Actor%20Object%20Reference)))

(event EventTick
  (params (DeltaSeconds :type Float%20%28single-precision%29))
  (bind _returnvalue (Transformation|GetActorLocation))
  (bind _returnvalue_2 (Transformation|GetActorLocation))
  (bind _returnvalue_3 (Transformation|GetActorLocation))
  (bind _bubble (Variables|Default|GetBubble))
  (bind _speed (Variables|Default|GetSpeed))
  (bind _returnvalue_4 (Math|Conversions|ToVector2D(Vector) _returnvalue))
  (bind _returnvalue_5 (Math|Conversions|ToVector2D(Vector) _returnvalue_2))
  (bind _returnvalue_6 (Transformation|GetActorLocation _bubble))
  (bind _returnvalue_7 (Math|Conversions|ToVector2D(Vector) _returnvalue_3))
  (bind _sphere (Variables|/Game/TopDown/Blueprints/Bubble/BP_Bubble.BP_Bubble_C|GetSphere _bubble))
  (bind _returnvalue_8 (Components|Sphere|GetScaledSphereRadius _sphere))
  (bind _returnvalue_9 (Math|Conversions|ToVector2D(Vector) _returnvalue_6))
  (bind _returnvalue_10 (- _returnvalue_9 _returnvalue_7))
  (bind (_outdir _outlength) (Class|KismetMathLibrary|ToDirectionandLength2D _returnvalue_10))
  (bind _returnvalue_11 (- _outlength _returnvalue_8))
  (bind _returnvalue_12 (* _outdir _returnvalue_11))
  (bind _returnvalue_13 (+ _returnvalue_12 _returnvalue_4))
  (bind (_outdir_2 _outlength_2) (Class|KismetMathLibrary|ToDirectionandLength2D _returnvalue_13))
  (bind _returnvalue_14 (* _outdir_2 _speed))
  (bind _returnvalue_15 (* _returnvalue_14 DeltaSeconds))
  (bind _returnvalue_16 (+ _returnvalue_5 _returnvalue_15))
  (if (Utilities|IsValid (Variables|Default|GetBubble))
    (if (> _outlength_2 1e+01)
      (Transformation|SetActorLocation (Math|Vector|MakeVector (.x _returnvalue_16) (.y _returnvalue_16) 0.0) false false))))

(fn ConstructionScript)