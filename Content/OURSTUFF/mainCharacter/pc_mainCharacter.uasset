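; Player character Blueprint that handles gamepad movement and opening the pause menu.
; Left stick input directly sets the movement component's velocity on the horizontal plane at a fixed speed, with the Y axis inverted, instead of using movement input.
; Gamepad Special Right, P or Escape pauses the game and adds a new PauseMenu widget tagged with the TopDownMap level name.
; BeginPlay moves the character to the world origin.
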(event EventBeginPlay
  (Transformation|SetActorLocation "0, 0, 0" false false))

(event Collision|EventActorBeginOverlap
  (params (OtherActor :type Actor%20Object%20Reference)))

(event EventTick
  (params (DeltaSeconds :type Float%20%28single-precision%29)))

(event Input|KeyboardEvents|Escape
  (params (Key :type Key%20Structure :default "None"))
  (:Pressed
    (Game|SetGamePaused true)
    (bind _returnvalue (UserInterface|CreateWidget "/Game/TopDown/Blueprints/UI/PauseMenu.PauseMenu_C"))
    (UserInterface|Viewport|AddtoViewport _returnvalue 0)))

(event Input|KeyboardEvents|P
  (params (Key :type Key%20Structure :default "None"))
  (:Pressed
    (Game|SetGamePaused true)
    (bind _returnvalue (UserInterface|CreateWidget "/Game/TopDown/Blueprints/UI/PauseMenu.PauseMenu_C"))
    (UserInterface|Viewport|AddtoViewport _returnvalue 0)))

(event Input|GamepadEvents|GamepadSpecialRight
  (params (Key :type Key%20Structure :default "None"))
  (:Pressed
    (Game|SetGamePaused true)
    (bind _returnvalue (UserInterface|CreateWidget "/Game/TopDown/Blueprints/UI/PauseMenu.PauseMenu_C"))
    (UserInterface|Viewport|AddtoViewport _returnvalue 0)))

(event Input|GamepadEvents|GamepadLeft2D
  (params (AxisValue :type Vector :default "0, 0, 0"))
  (bind (_x _y) (Math|Vector|BreakVector AxisValue))
  (Variables|/Script/Engine.MovementComponent|SetVelocity (Variables|Character|GetCharacterMovement) (* (Math|Vector|MakeVector _x (* _y -1.0) 0.0) 4e+02)))

(fn ConstructionScript)