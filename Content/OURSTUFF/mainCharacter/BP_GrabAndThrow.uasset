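; BP_GrabAndThrow lets its owning actor, likely the main character, pick up and drop BP_Pickupable items with Space or the gamepad's right face button.
; A press while empty-handed runs a tall, narrow box overlap around the owner, then attaches the first item found and snaps it in front.
; A press while holding detaches the item in place; despite the name, no throw force is applied.
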(event EventBeginPlay)

(event EventTick
  (params (DeltaSeconds :type Float%20%28single-precision%29)))

(event Input|KeyboardEvents|SpaceBar
  (params (Key :type Key%20Structure))
  (bind _returnvalue (Components|GetOwner))
  (:Pressed
    (if (Variables|Default|GetHolding)
      ;[0.15 0.15 0.15 0.5] Let go of held item
      (Variables|Default|SetHolding false)
      (Transformation|DetachFromActor (Variables|Default|GetItemHeld) "KeepWorld" "KeepWorld" "KeepWorld")
      (else
        ;[0.15 0.15 0.15 0.5] Grab item
        (bind _outactors (Collision|BoxOverlapActors (Transformation|GetActorLocation _returnvalue) "50.000000,50.000000,10000.000000" (Utilities|Array|MakeArray "ObjectTypeQuery2") "/Game/OURSTUFF/Plants/BP_Pickupable.BP_Pickupable_C" (Utilities|Array|MakeArray _returnvalue) :!class /Script/Engine.KismetSystemLibrary))
        (if (Utilities|Array|IsNotEmpty _outactors)
          (Variables|Default|SetHolding true)
          (Variables|Default|SetItemHeld (Utilities|Array|Get(acopy) _outactors))
          (Transformation|AttachActorToActor (Utilities|Array|Get(acopy) _outactors) (Components|GetOwner) "None" "KeepRelative" "KeepRelative" "KeepWorld" false)
          (Transformation|SetRelativeLocation (Variables|/Script/Engine.Actor|GetRootComponent (Utilities|Array|Get(acopy) _outactors)) "70.000000,0.000000,0.000000" false true))))))

(event Input|GamepadEvents|GamepadFaceButtonRight
  (params (Key :type Key%20Structure))
  (bind _returnvalue (Components|GetOwner))
  (:Pressed
    (if (Variables|Default|GetHolding)
      ;[0.15 0.15 0.15 0.5] Let go of held item
      (Variables|Default|SetHolding false)
      (Transformation|DetachFromActor (Variables|Default|GetItemHeld) "KeepWorld" "KeepWorld" "KeepWorld")
      (else
        ;[0.15 0.15 0.15 0.5] Grab item
        (bind _outactors (Collision|BoxOverlapActors (Transformation|GetActorLocation _returnvalue) "50.000000,50.000000,10000.000000" (Utilities|Array|MakeArray "ObjectTypeQuery2") "/Game/OURSTUFF/Plants/BP_Pickupable.BP_Pickupable_C" (Utilities|Array|MakeArray _returnvalue) :!class /Script/Engine.KismetSystemLibrary))
        (if (Utilities|Array|IsNotEmpty _outactors)
          (Variables|Default|SetHolding true)
          (Variables|Default|SetItemHeld (Utilities|Array|Get(acopy) _outactors))
          (Transformation|AttachActorToActor (Utilities|Array|Get(acopy) _outactors) (Components|GetOwner) "None" "KeepRelative" "KeepRelative" "KeepWorld" false)
          (Transformation|SetRelativeLocation (Variables|/Script/Engine.Actor|GetRootComponent (Utilities|Array|Get(acopy) _outactors)) "70.000000,0.000000,0.000000" false true))))))